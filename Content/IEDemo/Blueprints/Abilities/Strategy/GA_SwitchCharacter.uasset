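; Gameplay ability that switches player control between the two playable characters, Fabien and Raffony.
; After committing, it branches on the avatar's CharacterSwitcher value and finds the other character by class in the level.
; It detaches that character's controller pending destroy, has the player controller possess it, and prints the switch.
; The previously played character then spawns its default controller before the ability ends.
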(event Ability|EventActivateAbility
  (bind _returnvalue (Game|GetPlayerController 0))
  (bind _returnvalue_2 (Ability|CommitAbility))
  (if _returnvalue_2
    (bind _asbp_base_playable_character (Utilities|Casting|CastToBP_BasePlayableCharacter (Ability|GetAvatarActorfromActorInfo)))
    (switch Utilities|FlowControl|Switch|SwitchonEnum_CharacterSwitcher (Variables|/Game/ThirdPerson/Blueprints/BP_BasePlayableCharacter.BP_BasePlayableCharacter_C|GetCharacterSwitcher _asbp_base_playable_character)
      (:NewEnumerator0
        (bind _outactors (Actor|GetAllActorsOfClass "/Game/ThirdPerson/Blueprints/BP_Raffony.BP_Raffony_C"))
        (Class|Pawn|DetachfromControllerPendingDestroy (Utilities|Array|Get(acopy) _outactors))
        (Variables|Default|SetPrevious%20Played%20Character (Game|GetPlayerCharacter 0))
        (Pawn|Possess _returnvalue (Utilities|Array|Get(acopy) _outactors))
        (Development|PrintText "Switch to Raffony" true true "(R=1.000000,G=0.285414,B=0.722536,A=1.000000)")
        (Pawn|SpawnDefaultController (Variables|Default|GetPrevious%20Played%20Character))
        (Ability|EndAbility))
      (:NewEnumerator1
        (bind _outactors_2 (Actor|GetAllActorsOfClass "/Game/ThirdPerson/Blueprints/BP_Fabien.BP_Fabien_C"))
        (Class|Pawn|DetachfromControllerPendingDestroy (Utilities|Array|Get(acopy) _outactors_2))
        (Variables|Default|SetPrevious%20Played%20Character (Game|GetPlayerCharacter 0))
        (Pawn|Possess _returnvalue (Utilities|Array|Get(acopy) _outactors_2))
        (Development|PrintText "Switch to Fabien" true true "(R=0.364583,G=0.213215,B=0.116245,A=1.000000)")
        (Pawn|SpawnDefaultController (Variables|Default|GetPrevious%20Played%20Character))
        (Ability|EndAbility)))
    (else
      (Ability|EndAbility))))

(event Ability|EventOnEndAbility
  (params (bWasCancelled :type Boolean)))