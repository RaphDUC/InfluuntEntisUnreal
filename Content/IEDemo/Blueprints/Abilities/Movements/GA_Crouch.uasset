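; GA_Crouch is a gameplay ability that makes the avatar Character crouch while the ability input is held.
; On activation it commits the ability, casts and caches the avatar as a Character, then crouches it and starts a WaitInputRelease task.
; Releasing the input uncrouches the character and ends the ability, and a failed commit or cast ends it immediately.
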(event Ability|EventActivateAbility
  (bind _returnvalue (Ability|CommitAbility))
  (if _returnvalue
    (bind _ascharacter (Utilities|Casting|CastToCharacter (Ability|GetAvatarActorfromActorInfo))
      (:then
        (Variables|Default|SetAvatarCharacter _ascharacter)
        (Ability|Tasks|WaitInputRelease false
          (:then
            (Character|Crouch (Variables|Default|GetAvatarCharacter)))
          (:OnRelease
            (Character|UnCrouch (Variables|Default|GetAvatarCharacter))
            (Ability|EndAbility))))
      (:CastFailed
        (Ability|EndAbility)))
    (else
      (Ability|EndAbility))))

(event Ability|EventOnEndAbility
  (params (bWasCancelled :type Boolean)))