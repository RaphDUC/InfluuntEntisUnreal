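; GA_Jump is a Gameplay Ability that makes the avatar Character jump.
; On activation it commits, calls Jump, and stops jumping when the input is released, allowing variable jump height.
; It stays active until an Event.Character.Landed gameplay event arrives, and ends at once if the commit or Character cast fails.
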(event Ability|EventActivateAbility
  (bind _returnvalue (Ability|CommitAbility))
  (if _returnvalue
    (bind _ascharacter (Utilities|Casting|CastToCharacter (Ability|GetAvatarActorfromActorInfo))
      (:then
        (Variables|Default|SetAvatarCharacter _ascharacter)
        (Ability|Tasks|WaitInputRelease false
          (:then
            (Character|Jump (Variables|Default|GetAvatarCharacter))
            (Ability|Tasks|WaitGameplayEvent "(TagName=\"Event.Character.Landed\")" 0
              (:then
                (Ability|EndAbility))))
          (:OnRelease
            (Character|StopJumping (Variables|Default|GetAvatarCharacter)))))
      (:CastFailed
        (Ability|EndAbility)))
    (else
      (Ability|EndAbility))))

(event Ability|EventOnEndAbility
  (params (bWasCancelled :type Boolean)))