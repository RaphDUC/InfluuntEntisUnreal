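; GA_Roll is a movement gameplay ability that makes the avatar character perform a simple forward roll.
; On activation it commits the ability, then launches the avatar Character along its forward vector, adding to existing velocity rather than overriding it.
; It prints a debug message and ends immediately, with no animation; a failed commit or cast also just ends the ability.
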(event Ability|EventActivateAbility
  (bind _returnvalue (Ability|CommitAbility))
  (if _returnvalue
    (bind _ascharacter (Utilities|Casting|CastToCharacter (Ability|GetAvatarActorfromActorInfo))
      (:then
        (Variables|Default|SetAvatarCharacter _ascharacter)
        (Character|LaunchCharacter (Variables|Default|GetAvatarCharacter) (* (Transformation|GetActorForwardVector (Variables|Default|GetAvatarCharacter)) 6e+02) false false)
        (Development|PrintString "Roll !" true true "(R=1.000000,G=0.376074,B=0.235953,A=1.000000)")
        (Ability|EndAbility))
      (:CastFailed
        (Ability|EndAbility)))
    (else
      (Ability|EndAbility))))

(event Ability|EventOnEndAbility
  (params (bWasCancelled :type Boolean)))